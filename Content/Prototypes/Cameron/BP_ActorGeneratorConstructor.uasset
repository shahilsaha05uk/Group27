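; Construction-time generator prototype that builds a road from spline meshes along a Spline component.
; When RenderRoad is on, the construction script divides the spline length by SpaceBetween and calls CreateRoad per segment through the Index variable.
; CreateRoad adds a RoadMesh spline mesh spanning that distance interval, with a normalized, spacing-scaled start tangent but no end tangent wired.
; CreateDecorations is an empty stub.
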(event `Create Decorations`)

(event `CreateRoad`
  (bind _spacebetween (`self.SpaceBetween`))
  (bind _spline (`self.Spline`))
  (bind _returnvalue (* (`self.Index`) _spacebetween))
  (bind _returnvalue_2 (`KismetMathLibrary.Conv_IntToDouble` _returnvalue))
  ;[1 1 1] Create Road
  (bind _returnvalue_3 (`AddComponent|NODE_AddSplineMeshComponent-3`))
  (`StaticMeshComponent.SetStaticMesh` _returnvalue_3 (`self.RoadMesh`))
  (`SplineMeshComponent.SetStartAndEnd` _returnvalue_3 (`SplineComponent.GetLocationAtDistanceAlongSpline` _spline _returnvalue_2 "Local") (* (`KismetMathLibrary.Normal` (`SplineComponent.GetTangentAtDistanceAlongSpline` _spline _returnvalue_2 "Local")) (`self.SpaceBetween`)) (`SplineComponent.GetLocationAtDistanceAlongSpline` _spline (+ _returnvalue _spacebetween) "Local") (0.0 0.0 0.0) true)
  (`SceneComponent.K2_AttachToComponent` _returnvalue_3 (`self.DefaultSceneRoot`) "None" "KeepRelative" "KeepRelative" "KeepRelative" true))

(fn `UserConstructionScript`
  (if (`self.RenderRoad`)
    (for _index (range (+ (`KismetMathLibrary.FTrunc` (/ (`SplineComponent.GetSplineLength` (`self.Spline`)) (`self.SpaceBetween`))) 1))
      (set `self.Index` _index)
      (`self.CreateRoad`))))