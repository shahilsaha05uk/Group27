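; Prototype actor that builds a road along its spline at BeginPlay, despite the generic ActorGenerator name.
; It loops over the spline points, adding a spline mesh component with RoadMesh for each, bent between that point and the next using local locations and tangents.
; The construction script is empty, so the road is generated only at runtime.
; Two disconnected loops hold unfinished distance-based spacing experiments using SpaceBetween and never run.
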(event `self.ReceiveBeginPlay`
  (for _index (range (+ (`SplineComponent.GetNumberOfSplinePoints` (`self.Spline`)) 1))
    (bind _returnvalue (`AddComponent|NODE_AddSplineMeshComponent-0`))
    (`StaticMeshComponent.SetStaticMesh` _returnvalue (`self.RoadMesh`))
    (bind (_location _tangent) (`SplineComponent.GetLocationAndTangentAtSplinePoint` (`self.Spline`) _index "Local"))
    (bind (_location_2 _tangent_2) (`SplineComponent.GetLocationAndTangentAtSplinePoint` (`self.Spline`) (+ _index 1) "Local"))
    (`SplineMeshComponent.SetStartAndEnd` _returnvalue _location _tangent _location_2 _tangent_2 true)))

(fn `UserConstructionScript`)