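; Prototype spline generator that builds a road and lines it with street lamps at BeginPlay, despite the constructor name.
; When RenderRoad is on, it tiles RoadMesh as spline mesh components, sized by the mesh's X bounds with length-normalized tangents.
; It spawns and attaches BP_Lamp actors every LampDistance, alternating sides at a perpendicular offset.
; EndPlay destroys every BP_Lamp in the world, and the Construction Script holds only disconnected road logic.
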(event `self.ReceiveBeginPlay`
  ;[1 1 1] Begin Play
  (`self.Road`)
  (`self.Lamp`))

(event `Road`
  (bind _segmentsize (`self.SegmentSize`))
  (bind _segmentsize_2 (`self.SegmentSize`))
  (bind _spline (`self.Spline`))
  (bind _returnvalue (`StaticMesh.GetBoundingBox` (`self.RoadMesh`)))
  (bind _returnvalue_2 (* (`self.Index`) _segmentsize))
  (bind _returnvalue_3 (`KismetMathLibrary.Conv_IntToDouble` _returnvalue_2))
  (bind _returnvalue_4 (+ _returnvalue_2 _segmentsize))
  (bind _returnvalue_5 (+ (`KismetMathLibrary.Abs` (.x (break `Box` _returnvalue))) (`KismetMathLibrary.Abs` (.x (`.Max` (break `Box` _returnvalue))))))
  ;[1 1 1] Road
  (if (`self.RenderRoad`)
    (set `self.SegmentSize` _returnvalue_5)
    (for _index (range (`KismetMathLibrary.FTrunc` (/ (`SplineComponent.GetSplineLength` (`self.Spline`)) _returnvalue_5)))
      (set `self.Index` _index)
      (bind _returnvalue_6 (`AddComponent|NODE_AddSplineMeshComponent-5`))
      (`StaticMeshComponent.SetStaticMesh` _returnvalue_6 (`self.RoadMesh`))
      (`SplineMeshComponent.SetStartAndEnd` _returnvalue_6 (`SplineComponent.GetLocationAtDistanceAlongSpline` _spline _returnvalue_3 "Local") (* (`KismetMathLibrary.Normal` (`SplineComponent.GetTangentAtDistanceAlongSpline` _spline _returnvalue_3 "World")) _segmentsize_2) (`SplineComponent.GetLocationAtDistanceAlongSpline` _spline _returnvalue_4 "Local") (* (`KismetMathLibrary.Normal` (`SplineComponent.GetTangentAtDistanceAlongSpline` _spline _returnvalue_4 "World")) _segmentsize_2) true)
      (`SceneComponent.K2_AttachToComponent` _returnvalue_6 (`self.DefaultSceneRoot`) "None" "KeepRelative" "KeepRelative" "KeepRelative" true))))

(event `Lamp`
  (bind _spline (`self.Spline`))
  (bind _lampdistancefrom (`self.LampDistanceFrom`))
  (bind _defaultsceneroot (`self.DefaultSceneRoot`))
  ;[1 1 1] Lamp
  (for _index (range (`KismetMathLibrary.FTrunc` (/ (`SplineComponent.GetSplineLength` (`self.Spline`)) (`self.LampDistance`))))
    (if (`self.RightSide`)
      (set `self.RightSide` false)
      (bind _returnvalue (`KismetMathLibrary.Conv_IntToDouble` (* (`self.LampDistance`) _index)))
      (bind _returnvalue_2 (`SplineComponent.GetTangentAtDistanceAlongSpline` _spline _returnvalue "Local"))
      (bind _returnvalue_3 (`KismetMathLibrary.Normal` (`KismetMathLibrary.RotateAngleAxis` _returnvalue_2 -90.0 (0.0 0.0 1.0))))
      (bind _returnvalue_4 (`SplineComponent.GetLocationAtDistanceAlongSpline` _spline _returnvalue "World"))
      (bind _returnvalue_5 (`|SpawnActorFromClass` "/Game/Prototypes/Cameron/Roads/BP_Lamp.BP_Lamp_C" (`KismetMathLibrary.MakeTransform` (+ (* _returnvalue_3 _lampdistancefrom) _returnvalue_4) (`KismetMathLibrary.NegateRotator` (`KismetMathLibrary.Conv_VectorToRotator` _returnvalue_3))) "Undefined" "MultiplyWithRoot" null null))
      (`self.K2_AttachToComponent` _returnvalue_5 _defaultsceneroot "None" "KeepWorld" "KeepRelative" "KeepRelative" true)
      (else
        (set `self.RightSide` true)
        (bind _returnvalue_6 (`KismetMathLibrary.Normal` (`KismetMathLibrary.RotateAngleAxis` _returnvalue_2 90.0 (0.0 0.0 1.0))))
        (bind _returnvalue_7 (`|SpawnActorFromClass` "/Game/Prototypes/Cameron/Roads/BP_Lamp.BP_Lamp_C" (`KismetMathLibrary.MakeTransform` (+ _returnvalue_4 (* _returnvalue_6 _lampdistancefrom)) (`KismetMathLibrary.NegateRotator` (`KismetMathLibrary.Conv_VectorToRotator` _returnvalue_6))) "Undefined" "MultiplyWithRoot" null null))
        (`self.K2_AttachToComponent` _returnvalue_7 _defaultsceneroot "None" "KeepWorld" "KeepRelative" "KeepRelative" true)))))

(event `self.ReceiveEndPlay`
  (params (EndPlayReason :type "EEndPlayReason Enum" :default "Destroyed"))
  (bind _outactors (`GameplayStatics.GetAllActorsOfClass` "/Game/Prototypes/Cameron/Roads/BP_Lamp.BP_Lamp_C"))
  (for _array_element _outactors
    (`self.K2_DestroyActor` _array_element)))

(fn `UserConstructionScript`)