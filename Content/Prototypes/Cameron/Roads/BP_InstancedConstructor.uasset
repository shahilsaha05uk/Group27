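; Prototype road constructor that populates an instanced static mesh component along a spline.
; When RenderRoad is set, the construction script adds one instance per SegmentSize of spline length.
; The instances receive no computed transform, as the spline location and tangent nodes are left unconnected.
; The CreateDecorations event is an empty stub.
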(event `Create Decorations`)

(fn `UserConstructionScript`
  (if (`self.RenderRoad`)
    (for _index (range (`KismetMathLibrary.FTrunc` (/ (`SplineComponent.GetSplineLength` (`self.Spline`)) (`self.SegmentSize`))))
      (set `self.Index` _index)
      (`InstancedStaticMeshComponent.AddInstance` (`self.InstancedStaticMesh`) (`KismetMathLibrary.MakeTransform` (0.0 0.0 0.0)) false))))