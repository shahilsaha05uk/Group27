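; BP_Road is a prototype road actor that builds its surface along a spline and populates it at play start.
; The construction script adds a spline mesh component between each pair of adjacent points, fitted to their local locations and tangents and scaled by RoadWidth.
; BeginPlay spawns actors, counted by NumberOfCars, spaced evenly by distance along the spline and rotated to follow it.
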(event `self.ReceiveBeginPlay`
  (bind _numberofcars (`self.NumberOfCars`))
  (bind _spline (`self.Spline`))
  (for _index (range (+ _numberofcars 1))
    (bind _returnvalue (`KismetMathLibrary.Lerp` 0.0 (`SplineComponent.GetSplineLength` (`self.Spline`)) (/ (- _index 1) _numberofcars)))
    (`|SpawnActorFromClass` "/Game/Prototypes/Griffyn/BP_Car.BP_Car_C" (`KismetMathLibrary.MakeTransform` (`SplineComponent.GetLocationAtDistanceAlongSpline` _spline _returnvalue "World") (`SplineComponent.GetRotationAtDistanceAlongSpline` _spline _returnvalue "World")) "Undefined" "MultiplyWithRoot" null null)))

(fn `Get Locations And Tangents`
  (params (SplinePoint :type Integer))
  (returns (StartLocation :type "Vector Structure") (StartTangent :type "Vector Structure") (EndLocation :type "Vector Structure") (EndTangent :type "Vector Structure"))
  (bind _spline (`self.Spline`))
  (bind (_location _tangent) (`SplineComponent.GetLocationAndTangentAtSplinePoint` _spline (+ SplinePoint 1) "Local"))
  (bind (_location_2 _tangent_2) (`SplineComponent.GetLocationAndTangentAtSplinePoint` _spline SplinePoint "Local"))
  (return _location_2 _tangent_2 _location _tangent))

(fn `UserConstructionScript`
  (bind _returnvalue (`KismetMathLibrary.MakeVector2D` (`self.RoadWidth`) 1.0))
  (for _index (range (+ (- (`SplineComponent.GetNumberOfSplinePoints` (`self.Spline`)) 2) 1))
    (bind _returnvalue_2 (`AddComponent|NODE_AddSplineMeshComponent-0`))
    (bind (_startlocation _starttangent _endlocation _endtangent) (`self.Get Locations And Tangents` _index))
    (`SplineMeshComponent.SetStartAndEnd` _returnvalue_2 _startlocation _starttangent _endlocation _endtangent true)
    (`SplineMeshComponent.SetStartScale` _returnvalue_2 _returnvalue true)
    (`SplineMeshComponent.SetEndScale` _returnvalue_2 _returnvalue true)))