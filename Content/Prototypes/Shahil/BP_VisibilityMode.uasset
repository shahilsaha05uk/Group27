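; Prototype game mode that sets up two local players, a helper and a player, when a new player starts.
; The starting controller is handled as the helper, and CreatePlayer adds a second controller for the player, each guarded by a validity check.
; InitController sends each controller a spawn message flagging whether it is the helper.
; An alternative path that spawns BP_Controller and assigns controller IDs is unconnected.
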(event `self.HandleStartingNewPlayer`
  (params (NewPlayer :type "PlayerController Object Reference"))
  (`self.SpawnHelper` NewPlayer)
  (`self.SpawnPlayer`))

(event `SpawnHelper`
  (params (HelperPC :type "PlayerController Object Reference"))
  (if (not (`KismetSystemLibrary.IsValid` (`self.HelperPC`)))
    (bind _output_get (set `self.HelperPC` HelperPC))
    (`self.InitController` _output_get true)))

(event `SpawnPlayer`
  (if (not (`KismetSystemLibrary.IsValid` (`self.PlayerPC`)))
    (bind _returnvalue (`GameplayStatics.CreatePlayer` -1))
    (bind _output_get (set `self.PlayerPC` _returnvalue))
    (`self.InitController` _output_get)))

(event `InitController`
  (params (Controller :type "PlayerController Object Reference") (SpawnHelper :type Boolean))
  (message `/Game/Prototypes/Shahil/BI_Controller.OnControllerSpawn` Controller SpawnHelper))

(fn `UserConstructionScript`)