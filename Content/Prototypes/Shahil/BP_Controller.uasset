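; Prototype controller that spawns and possesses either a Helper or a Player pawn, chosen by a SpawnHelper flag.
; OnControllerSpawn destroys any pawn it currently controls, then calls SpawnPawn.
; SpawnPawn creates the chosen class at the game mode's FindPlayerStart transform, stores it in MPlayer and possesses it.
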(event `SpawnPawn`
  (params (SpawnHelper :type Boolean))
  (if SpawnHelper
    (bind _returnvalue (`|SpawnActorFromClass` "/Game/Prototypes/Shahil/Helper.Helper_C" (`self.GetTransform` (`GameModeBase.K2_FindPlayerStart` (`GameplayStatics.GetGameMode`) self "")) "Undefined" "MultiplyWithRoot" null null))
    (bind _output_get (set `self.mPlayer` _returnvalue))
    (`self.Possess` _output_get)
    (else
      (bind _returnvalue_2 (`|SpawnActorFromClass` "/Game/Prototypes/Shahil/Player.Player_C" (`self.GetTransform` (`GameModeBase.K2_FindPlayerStart` (`GameplayStatics.GetGameMode`) self "")) "Undefined" "MultiplyWithRoot" null null))
      (bind _output_get_2 (set `self.mPlayer` _returnvalue_2))
      (`self.Possess` _output_get_2))))

(event `/Game/Prototypes/Shahil/BI_Controller.OnControllerSpawn`
  (params (bSpawnHelper :type Boolean))
  (bind _returnvalue (`self.K2_GetPawn`))
  (`/Engine/EditorBlueprintResources/StandardMacros.IsValid` _returnvalue
    (:`Is Valid`
      (`self.K2_DestroyActor` _returnvalue))
    (:`Is Not Valid`
      _))
  (`self.SpawnPawn` bSpawnHelper))

(fn `UserConstructionScript`)