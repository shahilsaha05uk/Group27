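; Prototype parkour climb component that decides whether a character can grab and hang from a ledge.
; AttemptToHang runs Detect and calls Hang, which is not defined here, only when both checks pass.
; Detect capsule-traces at the ledge collider on separate channels, first a short upward sweep for a platform, then an in-place check for a ledge.
; Traces draw debug shapes, successes print messages, and hit results go unused.
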(event `self.AttemptToHang`
  (bind _returnvalue (`self.Detect`))
  (if _returnvalue
    (`self.Hang`)
    (`KismetSystemLibrary.PrintString` "Attempt to hang")))

(fn `Detect`
  (returns (ReturnValue :type Boolean))
  (bind _mledgecollider (`self.mLedgeCollider`))
  (bind _returnvalue (`SceneComponent.K2_GetComponentLocation` _mledgecollider))
  (`|ExecutionSequence`
    (:`then_0`
      (bind (_hit _returnvalue_2) (`self.TraceForAValidPlatform` _returnvalue (+ _returnvalue (* (`SceneComponent.GetUpVector` _mledgecollider) 5.0))))
      (if _returnvalue_2
        (`KismetSystemLibrary.PrintString` "Building found!!")
        (else
          (return false))))
    (:`then_1`
      (bind (_hit_2 _returnvalue_3) (`self.TraceForAValidLedge` _returnvalue _returnvalue))
      (if _returnvalue_3
        (`KismetSystemLibrary.PrintString` "Ledge found!!")
        (else
          (return false))))
    (:`then_2`
      (return true))))

(fn `TraceForAValidLedge`
  (params (Start :type "Vector Structure") (End :type "Vector Structure"))
  (returns (hit :type "HitResult Structure") (ReturnValue :type Boolean))
  (bind (_outhit _returnvalue) (`KismetSystemLibrary.CapsuleTraceSingle` :`Start` Start :`End` End :`Radius` (`self.mLedgeDetectionCapsuleRadius`) :`HalfHeight` (`self.mLedgeDetectionCapsuleHeight`) :`TraceChannel` "TraceTypeQuery4" :`DrawDebugType` "ForDuration" :`TraceColor` (struct :`R` 1.0 :`G` 0.952515 :`A` 1.0)))
  (return _outhit _returnvalue))

(fn `TraceForAValidPlatform`
  (params (Start :type "Vector Structure") (End :type "Vector Structure"))
  (returns (hit :type "HitResult Structure") (ReturnValue :type Boolean))
  ;[0 0 0] Check for a valid platform
  (bind (_outhit _returnvalue) (`KismetSystemLibrary.CapsuleTraceSingle` :`Start` Start :`End` End :`Radius` (`self.mPlatformDetectionCapsuleRadius`) :`HalfHeight` (`self.mPlatformDetectionCapsuleHeight`) :`TraceChannel` "TraceTypeQuery5" :`DrawDebugType` "ForDuration"))
  (return _outhit _returnvalue))