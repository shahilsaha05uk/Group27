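; BP_Platforms is a parkour prototype platform that owns climbable ledges and tracks which is nearest the player.
; An editor-only event spawns and attaches BP_Ledge actors, and another initializes them with the platform as owner.
; Start/stop tracking events store the player and fire callbacks, while ledges register as candidates.
; Player location updates pick the nearest candidate and call SelectMessage on it; the looping search timer is left unwired.
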(event `SpawnLedge`
  ;[1 1 1] EDITOR ONLY!!
  (bind _returnvalue (`|SpawnActorFromClass` "/Game/Prototypes/Shahil/Parkour/BP_Ledge.BP_Ledge_C" (`KismetMathLibrary.MakeTransform` (0.0 -50.0 0.0)) "Undefined" "MultiplyWithRoot" self null))
  (`self.K2_AttachToActor` _returnvalue self "None" "KeepRelative" "KeepRelative" "KeepWorld" true)
  (`KismetArrayLibrary.Array_Add` (`self.Ledges`) _returnvalue))

(event `UpdateLedgeInits`
  ;[1 1 1] EDITOR ONLY!!
  (for _array_element (`self.Ledges`)
    (`/Game/Prototypes/Shahil/Parkour/BP_Ledge.Init` _array_element self)))

(event `self.UpdateBuildingLedgeAvailability`
  (params (PlayerRef :type "Actor Object Reference"))
  (message `LedgeInterface.Select` (`.ReturnValue` (`GameplayStatics.FindNearestActor` (`self.K2_GetActorLocation` PlayerRef) (`self.ClosestLedgesToPlayer`))) false))

(event `self.StartTrackingPlayer`
  (params (playerRef :type "Actor Object Reference"))
  (bind _output_get (set `self.Player Ref` playerRef))
  (`self.OnStartTrackingPlayer` _output_get))

(event `self.StopTrackingPlayer`
  (`self.OnStopTrackingPlayer`)
  (set `self.Player Ref` null)
  (`KismetArrayLibrary.Array_Clear` (`self.ClosestLedgesToPlayer`)))

(event `RegisterLedge`
  (params (NewItem :type "Actor Object Reference (by ref)"))
  (`KismetArrayLibrary.Array_AddUnique` (`self.ClosestLedgesToPlayer`) NewItem))

(event `DeregisterLedge`
  (params (Item :type "Actor Object Reference (by ref)"))
  (bind _closestledgestoplayer (`self.ClosestLedgesToPlayer`))
  (if (`KismetArrayLibrary.Array_Contains` _closestledgestoplayer Item)
    (`KismetArrayLibrary.Array_RemoveItem` _closestledgestoplayer Item)))

(event `StartTrackingForTheClosestLedgeToThePlayer`
  (`/Engine/EditorBlueprintResources/StandardMacros.IsValid` (`self.Player Ref`)))

(event `StartSearch`
  (bind _closestledge (`self.ClosestLedge`))
  (if (and (`KismetSystemLibrary.IsValid` _closestledge) (`KismetArrayLibrary.Array_Contains` (`self.ClosestLedgesToPlayer`) _closestledge))
    (bind _returnvalue (`self.GetClosestLedge`))
    (set `self.ClosestLedge` _returnvalue)))

(event `PlayerLocationUpdated`
  (`/Engine/EditorBlueprintResources/StandardMacros.IsValid` (`self.Player Ref`)
    (:`Is Valid`
      (bind _returnvalue (`self.GetClosestLedge`))
      (set `self.ClosestLedge` _returnvalue))))

(event `StopTrackingForTheClosestLedgeToThePlayer`
  (`KismetSystemLibrary.K2_ClearAndInvalidateTimerHandle` (`self.ClosestLedgeSearchTimeHandler`)))

(fn `GetBuildingMesh`
  (returns (Mesh :type "StaticMeshComponent Object Reference"))
  (return null))

(fn `GetClosestLedge`
  (returns (ReturnValue :type "Actor Object Reference"))
  (bind _closestledgestoplayer (`self.ClosestLedgesToPlayer`))
  (bind (_distance _returnvalue) (`GameplayStatics.FindNearestActor` (`self.K2_GetActorLocation` (`self.Player Ref`)) _closestledgestoplayer))
  (if (`KismetArrayLibrary.Array_IsNotEmpty` _closestledgestoplayer)
    (message `LedgeInterface.Select` _returnvalue false)
    (return _returnvalue)))

(fn `GetLedges`
  (returns (ReturnValue :type "Array of Actor Object Reference"))
  (return (`self.Ledges`)))

(fn `UserConstructionScript`)