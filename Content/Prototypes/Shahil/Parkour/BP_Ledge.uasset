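; Parkour prototype ledge actor that swaps materials to show highlighted, selected or standable states.
; Init binds it to its building's player-tracking events, and tracking runs on a fast looping timer rather than Tick.
; Threshold-range changes toggle the highlight and register or deregister the ledge with the building, drawing a debug line on activation.
; The distance helper's calculation is unconnected, and the OnLedgeUpdate binding never runs.
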(event `self.Select`
  (params (isStandable :type Boolean))
  (if isStandable
    (`PrimitiveComponent.SetMaterial` (`self.ledge`) 0 (`self.standableMat`))
    (else
      (`PrimitiveComponent.SetMaterial` (`self.ledge`) 0 (`self.selectedMat`)))))

(event `self.Deselect`
  (`PrimitiveComponent.SetMaterial` (`self.ledge`) 0 (`self.normalMat`)))

(event `self.Highlight`
  (`PrimitiveComponent.SetMaterial` (`self.ledge`) 0 (`self.highlightMat`)))

(event `self.Dehighlight`
  (`PrimitiveComponent.SetMaterial` (`self.ledge`) 0 (`self.normalMat`)))

(event `Init`
  (params (BuildingRef :type "/Game/Prototypes/Shahil/Parkour/BP_Platforms Object Reference"))
  (bind _output_get (set `self.BuildingRef` BuildingRef))
  (add `/Game/Prototypes/Shahil/Parkour/BP_Platforms.OnStartTrackingPlayer` _output_get (`|CreateDelegate` :!event `StartTracking`))
  (add `/Game/Prototypes/Shahil/Parkour/BP_Platforms.OnStopTrackingPlayer` _output_get (`|CreateDelegate` :!event `StopTracking`)))

(event `OnLedgeUpdate`
  (params (PlayerRef :type "Actor Object Reference"))
  (if (<= (`KismetMathLibrary.Vector_Distance` (`self.K2_GetActorLocation` PlayerRef) (`self.K2_GetActorLocation`)) (`self.thresholdRange`))
    (`self.Highlight`)
    (else
      (`self.Dehighlight`))))

(event `StartTracking`
  (params (PlayerRef :type "Actor Object Reference"))
  (set `self.PlayerRef` PlayerRef)
  (bind _output_get (set `self.CurrentDistance` (`self.getDistanceFromThePlayer`)))
  (set `self.LastDistance` _output_get)
  (bind _returnvalue (`KismetSystemLibrary.K2_SetTimerDelegate` (`|CreateDelegate` :!event `Tracking`) 0.005 true))
  (set `self.PlayerTrackingTimeHandler` _returnvalue))

(event `StopTracking`
  (`KismetSystemLibrary.K2_ClearAndInvalidateTimerHandle` (`self.PlayerTrackingTimeHandler`))
  (set `self.PlayerRef` null)
  (`self.Dehighlight`))

(event `Tracking`
  (if (> (`self.distanceDifference`) (`KismetMathLibrary.Abs` (- (`self.getDistanceFromThePlayer`) (`self.LastDistance`))))
    (`self.PlayerLocationUpdated`))
  (bind _output_get (set `self.mShouldActivate` (<= (`self.CurrentDistance`) (`self.thresholdRange`))))
  (if (!= _output_get (`self.mLastStatus`))
    (set `self.mLastStatus` (`self.mShouldActivate`))
    (`self.UpdateState`)))

(event `UpdateState`
  (if (`self.mShouldActivate`)
    (`KismetSystemLibrary.DrawDebugLine` (`self.K2_GetActorLocation`) (`self.K2_GetActorLocation` (`self.PlayerRef`)) (struct) 5.0 1.0)
    (`self.Highlight`)
    (`/Game/Prototypes/Shahil/Parkour/BP_Platforms.RegisterLedge` (`self.BuildingRef`) self)
    (elif (<= (`self.CurrentDistance`) (`self.thresholdRange`))
      (`self.Highlight`)
      (else
        (`self.Dehighlight`)
        (`/Game/Prototypes/Shahil/Parkour/BP_Platforms.DeregisterLedge` (`self.BuildingRef`) self)))))

(event `PlayerLocationUpdated`
  (`self.UpdateState`)
  (set `self.LastDistance` (`self.CurrentDistance`))
  (`/Game/Prototypes/Shahil/Parkour/BP_Platforms.PlayerLocationUpdated` (`self.BuildingRef`)))

(fn `GetBuildingRef`
  (returns (ReturnValue :type "Actor Object Reference"))
  (return (`self.BuildingRef`)))

(fn `UserConstructionScript`)