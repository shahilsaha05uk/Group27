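; Powerup that extends the pizza timer by raising the quality of every order in the customer subsystem's order list.
; On activation it loops over the order map's values and calls AddQuality with IncreaseBy on each.
; It then deactivates by clearing CollidedActor; with an empty order list, activation does nothing and skips that deactivation.
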(event `self.ActivatePowerup`
  (bind _returnvalue (`CustomerSubsystem.GetOrderList` (subsystem `CustomerSubsystem`)))
  (if (> (`BlueprintMapLibrary.Map_Length` _returnvalue) 0)
    (bind _values (`BlueprintMapLibrary.Map_Values` _returnvalue))
    (for _array_element _values
      (`CustomerMarker.AddQuality` _array_element (`self.Increase By`)))
    (`self.DeactivatePowerup`)))

(event `self.DeactivatePowerup`
  (set `self.collidedActor` null))

(fn `UserConstructionScript`
  (`parent.UserConstructionScript`))