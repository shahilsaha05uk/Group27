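; Shop trigger that starts pizza order rounds and the day when a parkour player enters, swapping floor material to show availability.
; The first round uses a plain collider; completing all orders starts a clock countdown and arms a countdown collider.
; Arriving in time stops the clock; expiry initiates orders as late, leaving late arrivals only to collect them.
; Clock, customer and calendar subsystems coordinate the loop alongside a pizza component.
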(event `self.CountdownCollider.OnComponentBeginOverlap`
  (params (OverlappedComponent :type "PrimitiveComponent Object Reference") (OtherActor :type "Actor Object Reference") (OtherComp :type "PrimitiveComponent Object Reference") (OtherBodyIndex :type Integer) (bFromSweep :type Boolean) (SweepResult :type "HitResult Structure (by ref)"))
  ;[0 0 0] Should trigger  the Order generation
  (if (`KismetSystemLibrary.DoesImplementInterface` OtherActor "/Script/GroupProj27.ParkourPlayerInterface")
    (switch `EClockStatus` (`ClockSubsystem.GetClockStatus` (subsystem `ClockSubsystem`))
      (:`TIMER_RUNNING`
        ;;[0 0 0] WITHIN TIME REACHED
        (`ClockSubsystem.StopTimer` (subsystem `ClockSubsystem`))
        (`self.InitOrders` OtherActor))
      (:`TIMER_FINISHED`
        ;;[0 0 0] IS LATE
        (`self.UpdateEntities` OtherActor)
        (`CustomerSubsystem.OnOrderInitialised` (subsystem `CustomerSubsystem`))))))

(event `self.NormalCollider.OnComponentBeginOverlap`
  (params (OverlappedComponent :type "PrimitiveComponent Object Reference") (OtherActor :type "Actor Object Reference") (OtherComp :type "PrimitiveComponent Object Reference") (OtherBodyIndex :type Integer) (bFromSweep :type Boolean) (SweepResult :type "HitResult Structure (by ref)"))
  ;[0 0 0] Should trigger  the Order generation
  ;;[0 0.04772 1] When the Normal Collider is enavled
  (if (`KismetSystemLibrary.DoesImplementInterface` OtherActor "/Script/GroupProj27.ParkourPlayerInterface")
    (`self.InitOrders` OtherActor)))

(event `InitOrders`
  (params (ActorRef :type "Object Object Reference"))
  ;[0 0 0] Initialise Orders for the player
  (`/Engine/EditorBlueprintResources/StandardMacros.IsValid` ActorRef
    (:`Is Valid`
      (`PizzaComponent.InitiateOrders` (`self.BP_PizzaComponent`) true)
      (`self.UpdateEntities` ActorRef))
    (:`Is Not Valid`
      (`KismetSystemLibrary.PrintString` "Late Arrival")
      (`PizzaComponent.InitiateOrders` (`self.BP_PizzaComponent`) false)))
  (`PizzaComponent.StartQualityTimer` (`self.BP_PizzaComponent`))
  (`CalenderSubsystem.StartDay` (subsystem `CalenderSubsystem`)))

(event `UpdateEntities`
  (params (Target :type "Object Object Reference"))
  (message `ParkourPlayerInterface.OnOrdersRequested` Target)
  (`self.ToggleShop` false)
  (`self.ToggleCollider` "NewEnumerator2"))

(event `self.ReceiveBeginPlay`
  (`self.InitBindings`)
  (`self.ToggleCollider` "NewEnumerator1")
  (`self.ToggleShop` true))

(event `ToggleCollider`
  (params (ColliderToEnable :type "/Game/Prototypes/Shahil/GameLoopFiles/EColliderToggle Enum" :default "NewEnumerator0"))
  ;[0 0 0] Toggle between two colliders
  (switch `/Game/Prototypes/Shahil/GameLoopFiles/EColliderToggle` ColliderToEnable
    (:`NewEnumerator0`
      (set `PrimitiveComponent.bGenerateOverlapEvents` true (`self.CountdownCollider`))
      (set `PrimitiveComponent.bGenerateOverlapEvents` false (`self.NormalCollider`)))
    (:`NewEnumerator1`
      (set `PrimitiveComponent.bGenerateOverlapEvents` false (`self.CountdownCollider`))
      (set `PrimitiveComponent.bGenerateOverlapEvents` true (`self.NormalCollider`)))
    (:`NewEnumerator2`
      (set `PrimitiveComponent.bGenerateOverlapEvents` false (`self.CountdownCollider`))
      (set `PrimitiveComponent.bGenerateOverlapEvents` false (`self.NormalCollider`)))
    (:`NewEnumerator3`
      (set `PrimitiveComponent.bGenerateOverlapEvents` true (`self.CountdownCollider`))
      (set `PrimitiveComponent.bGenerateOverlapEvents` true (`self.NormalCollider`)))))

(event `OnOrdersCompleted`
  (params (ID :type Integer) (RemainingOrders :type Integer))
  (set `self.bHasReached` false)
  (if (<= RemainingOrders 0)
    (`ClockSubsystem.StartTimer` (subsystem `ClockSubsystem`))
    (`self.ToggleShop` true)
    (`self.ToggleCollider` "NewEnumerator0")))

(event `ToggleShop`
  (params (Activate :type Boolean))
  ;[0 0 0] Toggle Shop Activation
  (if Activate
    (`PrimitiveComponent.SetMaterial` (`self.Plane`) 0 (`self.ActivatedMat`))
    (else
      (`PrimitiveComponent.SetMaterial` (`self.Plane`) 0 (`self.DeactivatedMat`)))))

(event `InitBindings`
  (`|ExecutionSequence`
    (:`then_0`
      ;[0 0 0] Binding to keep track of when an order is collected by the customer
      (add `CustomerSubsystem.OnOrderCollected` (subsystem `CustomerSubsystem`) (`|CreateDelegate` :!event `OnOrdersCompleted`)))
    (:`then_1`
      ;[0 0 0] Clock
      (add `ClockSubsystem.FinishTimer` (subsystem `ClockSubsystem`) (`|CreateDelegate` :!event `FinishTimer`)))))

(event `FinishTimer`
  (`self.InitOrders` null))

(fn `UserConstructionScript`)