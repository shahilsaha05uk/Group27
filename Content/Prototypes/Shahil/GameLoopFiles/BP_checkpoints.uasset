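; BP_checkpoints is a customer checkpoint in the pizza game loop prototype that registers itself with the Customer Subsystem by ID on BeginPlay.
; ToggleCustomer switches it on or off by swapping the plane material, setting the active flag and toggling the sphere's overlap events.
; When an actor implementing ParkourPlayerInterface enters the active sphere, CollectPizza deactivates the checkpoint and reports the collected order to the subsystem.
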(event `self.ReceiveBeginPlay`
  (`CustomerSubsystem.RegisterCustomer` (subsystem `CustomerSubsystem`) (`self.CustomerID`) self))

(event `self.Sphere.OnComponentBeginOverlap`
  (params (OverlappedComponent :type "PrimitiveComponent Object Reference") (OtherActor :type "Actor Object Reference") (OtherComp :type "PrimitiveComponent Object Reference") (OtherBodyIndex :type Integer) (bFromSweep :type Boolean) (SweepResult :type "HitResult Structure (by ref)"))
  (if (and (`KismetSystemLibrary.DoesImplementInterface` OtherActor "/Script/GroupProj27.ParkourPlayerInterface") (`self.bIsActivated`))
    (`self.CollectPizza`)))

(event `self.ToggleCustomer`
  (params (Value :type Boolean))
  (bind _sphere (`self.Sphere`))
  ;[1 0.7661 0] DEBUG!!
  (if Value
    (`PrimitiveComponent.SetMaterial` (`self.Plane`) 0 (`self.activatedMat`))
    (set `self.bIsActivated` true)
    (set `PrimitiveComponent.bGenerateOverlapEvents` true _sphere)
    (else
      (`PrimitiveComponent.SetMaterial` (`self.Plane`) 0 (`self.deActivatedMat`))
      (set `self.bIsActivated` false)
      (set `PrimitiveComponent.bGenerateOverlapEvents` false _sphere))))

(event `self.CollectPizza`
  (`self.ToggleCustomer` false)
  (`CustomerSubsystem.OrderCollected` (subsystem `CustomerSubsystem`) (`self.CustomerID`)))

(fn `UserConstructionScript`)