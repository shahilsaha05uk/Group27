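; BP_Enemy is a stealth prototype AI enemy that supplies looping patrol points from a referenced waypoint actor.
; On BeginPlay it copies that actor's waypoint list and, if it is not empty, resets the index and calls RunBTMessage on its controller.
; GetNextWaypoint returns each point in turn, converted from the waypoint actor's local space to world space, and wraps back to the first after the last.
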(event `self.ReceiveBeginPlay`
  (bind _output_get (set `self.Waypoints` (`/Game/Prototypes/Shahil/Stealth/AI/BP_Waypoint.Waypoints` (`self.WaypointRef`))))
  (bind _returnvalue (`KismetArrayLibrary.Array_Length` _output_get))
  (if (> _returnvalue 0)
    (set `self.totalWaypoints` _returnvalue)
    (set `self.currentWaypointIndex` 0)
    (message `/Game/Prototypes/Shahil/Stealth/AI/BI_EnemyController.RunBT` (`self.GetController`))))

(fn `getNextWaypoint`
  (returns (Value :type "Vector Structure"))
  (if (not (< (`self.currentWaypointIndex`) (`self.totalWaypoints`)))
    (set `self.currentWaypointIndex` 0))
  (set `self.currentWaypoint` (`KismetMathLibrary.TransformLocation` (`self.GetTransform` (`self.WaypointRef`)) (`|GetArrayItem` (`self.Waypoints`) (`self.currentWaypointIndex`))))
  (bind _result (`/Engine/EditorBlueprintResources/StandardMacros.IncrementInt` (`self.currentWaypointIndex`))
    (:`  `
      (set `self.currentWaypointIndex` _result)
      (return (`self.currentWaypoint`)))))

(fn `UserConstructionScript`)