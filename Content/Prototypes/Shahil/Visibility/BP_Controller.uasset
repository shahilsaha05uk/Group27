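; BP_Controller is a prototype player controller that lets one player switch between a helper pawn and a ghost pawn.
; On BeginPlay it adds the default Enhanced Input mapping context, then spawns both pawns at the player start chosen by the game mode and possesses the helper.
; Hard-wired G and H keys unpossess the current pawn and possess the stored ghost or helper respectively.
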(event `SpawnPawn`
  (params (SpawnHelper :type Boolean))
  (if SpawnHelper
    (bind _returnvalue (`|SpawnActorFromClass` "/Game/Prototypes/Shahil/Visibility/BP_HelperPlayer.BP_HelperPlayer_C" (`self.GetTransform` (`GameModeBase.K2_FindPlayerStart` (`GameplayStatics.GetGameMode`) self "")) "Undefined" "MultiplyWithRoot" null null))
    (bind _output_get (set `self.mHelperPlayer` _returnvalue))
    (`self.Possess` _output_get)
    (else
      (bind _returnvalue_2 (`|SpawnActorFromClass` "/Game/Prototypes/Shahil/Visibility/BP_GhostPlayer.BP_GhostPlayer_C" (`self.GetTransform` (`GameModeBase.K2_FindPlayerStart` (`GameplayStatics.GetGameMode`) self "")) "Undefined" "MultiplyWithRoot" null null))
      (set `self.mGhostPlayer` _returnvalue_2))))

(event `/Game/Prototypes/Shahil/Visibility/BI_Controller.OnControllerSpawn`
  (`self.SpawnPawn` true)
  (`self.SpawnPawn` false))

(event `Key|G`
  (params (Key :type "Key Structure"))
  (:`Pressed`
    (`self.UnPossess`)
    (`self.Possess` (`self.mGhostPlayer`))))

(event `Key|H`
  (params (Key :type "Key Structure"))
  (:`Pressed`
    (`self.UnPossess`)
    (`self.Possess` (`self.mHelperPlayer`))))

(event `self.ReceiveBeginPlay`
  (`EnhancedInputSubsystemInterface.AddMappingContext` (subsystem `EnhancedInputLocalPlayerSubsystem`) "/Game/ThirdPerson/Input/IMC_Default.IMC_Default" 0 (struct))
  (`/Game/Prototypes/Shahil/Visibility/BI_Controller.OnControllerSpawn`))

(fn `UserConstructionScript`)