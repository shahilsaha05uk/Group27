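; Parent projectile for AI that damages the player's orders on contact.
; On BeginPlay it sets a suggested toss velocity aimed at the Target's predicted position, leading it by distance over launch speed times target velocity.
; The projectile rotates to follow its velocity, with trajectory debug drawing enabled.
; Overlapping an actor that implements ParkourPlayerInterface deals damage to orders through the CustomerSubsystem and destroys the projectile.
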(event `self.ReceiveBeginPlay`
  (bind (_startpos _endpos _launchspeed) (`self.CalculateProjectileVelocity`))
  (bind _projectilemovement (`self.ProjectileMovement`))
  ;[0 0 0] Calculate the Velocity on Begin play
  (bind _tossvelocity (`GameplayStatics.BlueprintSuggestProjectileVelocity` _startpos _endpos _launchspeed 0.0 "DoNotTrace" 0.0 false true))
  (set `MovementComponent.Velocity` _tossvelocity _projectilemovement)
  (set `ProjectileMovementComponent.bRotationFollowsVelocity` true _projectilemovement))

(event `self.Collider.OnComponentBeginOverlap`
  (params (OverlappedComponent :type "PrimitiveComponent Object Reference") (OtherActor :type "Actor Object Reference") (OtherComp :type "PrimitiveComponent Object Reference") (OtherBodyIndex :type Integer) (bFromSweep :type Boolean) (SweepResult :type "HitResult Structure (by ref)"))
  ;[0 0 0] When the Projectile overlaps, it deals damage to the orders, and Destroys
  (if (`KismetSystemLibrary.DoesImplementInterface` OtherActor "/Script/GroupProj27.ParkourPlayerInterface")
    (`CustomerSubsystem.DealDamageToOrders` (subsystem `CustomerSubsystem`) (`self.DamageValue`))
    (`self.K2_DestroyActor`)))

(fn `UserConstructionScript`)