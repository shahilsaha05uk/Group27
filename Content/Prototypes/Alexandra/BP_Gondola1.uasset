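; BP_Gondola1 is a prototype gondola actor that travels along a spline path in the level.
; On BeginPlay it finds a BP_Path1 actor by class, stores it as Path and calls StartMoving.
; A Timeline's Alpha maps to distance along the full spline length, and each update sets the gondola's location and rotation from the world-space spline transform at that distance.
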(event `self.ReceiveBeginPlay`
  (bind _returnvalue (`GameplayStatics.GetActorOfClass` "/Game/Prototypes/Alexandra/BP_Path1.BP_Path1_C"))
  (set `self.Path` _returnvalue)
  (`self.Start Moving`))

(event `Start Moving`
  (bind (_direction _alpha) (`Timeline|Timeline`)
    (:`Update`
      (bind (_returnvalue_location _returnvalue_rotation) (`KismetMathLibrary.BreakTransform` (`SplineComponent.GetTransformAtDistanceAlongSpline` (`/Game/Prototypes/Alexandra/BP_Path1.Spline` (`self.Path`)) (`KismetMathLibrary.Lerp` 0.0 (`SplineComponent.GetSplineLength` (`/Game/Prototypes/Alexandra/BP_Path1.Spline` (`self.Path`))) _alpha) "World" false)))
      (`self.K2_SetActorLocationAndRotation` _returnvalue_location _returnvalue_rotation))))

(fn `UserConstructionScript`)