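; BP_Gondola2 is a prototype gondola actor that travels along a spline path on its own once play begins.
; On BeginPlay it finds the BP_Path2 actor in the level and starts a Timeline.
; Each update maps the Timeline alpha to a distance along the path's spline, then sets the gondola's world location and rotation to that point.
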(event `self.ReceiveBeginPlay`
  (bind _returnvalue (`GameplayStatics.GetActorOfClass` "/Game/Prototypes/Alexandra/BP/BP_Path2.BP_Path2_C"))
  (set `self.Path` _returnvalue)
  (`self.Start Moving`))

(event `Start Moving`
  (bind (_direction _alpha) (`Timeline|Timeline`)
    (:`Update`
      (bind (_returnvalue_location _returnvalue_rotation) (`KismetMathLibrary.BreakTransform` (`SplineComponent.GetTransformAtDistanceAlongSpline` (`/Game/Prototypes/Alexandra/BP/BP_Path2.Spline` (`self.Path`)) (`KismetMathLibrary.Lerp` 0.0 (`SplineComponent.GetSplineLength` (`/Game/Prototypes/Alexandra/BP/BP_Path2.Spline` (`self.Path`))) _alpha) "World" false)))
      (`self.K2_SetActorLocationAndRotation` _returnvalue_location _returnvalue_rotation))))

(fn `UserConstructionScript`)