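; BPC_MinimapPOI is a component that marks its owning actor as a point of interest on the minimap.
; InitialisePOI takes the parent player, caches its HUD and minimap widget, then has that widget create an icon for the owner.
; A class check for BP_checkpoints after icon creation and the RemovePOI event are both empty stubs.
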(event `/Game/StudentWork/BPI_InitialisePOI.InitialisePOI`
  (params (`Parent Player` :type "/Game/BP/BP_ParentPlayer Object Reference"))
  (bind _output_get (set `self.Parent Player` `Parent Player`))
  (bind _output_get_2 (set `self.HUD` (`/Game/BP/BP_ParentPlayer.HUD` _output_get)))
  (set `self.WBP Minimap` (`/Game/Widgets/WBP_PlayerHUD.WBP_Minimap` _output_get_2))
  (`self.Create POI Icon`))

(event `Create POI Icon`
  (bind _returnvalue (`self.GetOwner`))
  (`/Game/StudentWork/UI/Map/WBP_MiniMap.Create POI Icon` (`self.WBP Minimap`) _returnvalue)
  (if (== (`GameplayStatics.GetObjectClass` _returnvalue) "/Game/Prototypes/Shahil/GameLoopFiles/BP_checkpoints.BP_checkpoints_C")
    _))

(event `/Game/StudentWork/BPI_InitialisePOI.RemovePOI`)