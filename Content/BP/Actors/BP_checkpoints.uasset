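; Pizza customer checkpoint actor that the player overlaps to hand over an order and earn balance.
; After a short delay on BeginPlay it registers with the customer subsystem, stores its ID and caches the player.
; ToggleCustomer switches material, particles and overlap events, and initialises the minimap POI when activated.
; An overlap by a ParkourPlayerInterface actor while active deactivates it, reports collection, adds balance and plays a sound.
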(event `self.ReceiveBeginPlay`
  ;[0 0 0] The Checkpoints marks attendance to the Subsystem
  (`KismetSystemLibrary.Delay` 0.5)
  (bind _returnvalue (`CustomerSubsystem.RegisterCustomer` (subsystem `CustomerSubsystem`) self))
  (set `self.CustomerID` _returnvalue)
  (bind _asbp_parent_player (cast `/Game/BP/BP_ParentPlayer` (`GameplayStatics.GetPlayerCharacter` 0)))
  (set `self.Player` _asbp_parent_player))

(event `self.Sphere.OnComponentBeginOverlap`
  (params (OverlappedComponent :type "PrimitiveComponent Object Reference") (OtherActor :type "Actor Object Reference") (OtherComp :type "PrimitiveComponent Object Reference") (OtherBodyIndex :type Integer) (bFromSweep :type Boolean) (SweepResult :type "HitResult Structure (by ref)"))
  ;[0 0 0] if the checkpoint is enabled, the customer has collected the pizza
  (if (and (`KismetSystemLibrary.DoesImplementInterface` OtherActor "/Script/GroupProj27.ParkourPlayerInterface") (`self.bIsActivated`))
    (`self.CollectPizza`)))

(event `self.CollectPizza`
  ;[0 0 0] When the Customer Collects the pizza...
  ; 1) De-activate this checkpoint
  ; 2) Let the Subsystem know this
  (`parent.CollectPizza`)
  (`self.ToggleCustomer` false)
  (`CustomerSubsystem.OrderCollected` (subsystem `CustomerSubsystem`) (`self.CustomerID`))
  (`ResourceSubsystem.AddBalance` (subsystem `ResourceSubsystem`) 1)
  (`GameplayStatics.PlaySound2D` (`self.MoneyCollectSound`) 1.0 1.0 0.0 null null))

(event `self.ToggleCustomer`
  (params (Value :type Boolean))
  (bind _activatedparticles (`self.activatedParticles`))
  (bind _sphere (`self.Sphere`))
  ;[0 0 0] DEBUG!!
  (if Value
    (`PrimitiveComponent.SetMaterial` (`self.Plane`) 0 (`self.activatedMat`))
    (set `self.bIsActivated` true)
    (set `PrimitiveComponent.bGenerateOverlapEvents` true _sphere)
    (`ActorComponent.Activate` _activatedparticles true)
    (message `/Game/StudentWork/BPI_InitialisePOI.InitialisePOI` (`self.BPC_MinimapPOI`) (`self.Player`))
    (else
      (`PrimitiveComponent.SetMaterial` (`self.Plane`) 0 (`self.deActivatedMat`))
      (set `self.bIsActivated` false)
      (set `PrimitiveComponent.bGenerateOverlapEvents` false _sphere)
      (`ActorComponent.Deactivate` _activatedparticles))))

(fn `UserConstructionScript`)