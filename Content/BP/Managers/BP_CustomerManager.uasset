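; Customer manager that spawns BP_checkpoints actors and registers them as customers under incrementing IDs.
; SpawnCustomers increments the ID, spawns a checkpoint actor and adds it to CustomerMap.
; BeginPlay assigns CustomerMap to the Customers map in CustomerListDataAsset, and EndPlay clears that data asset map.
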(event `SpawnCustomers`
  (bind _result (`/Engine/EditorBlueprintResources/StandardMacros.IncrementInt` (`self.id`))
    (:`  `
      (set `self.id` _result)
      (bind _returnvalue (`|SpawnActorFromClass` "/Game/Prototypes/Shahil/GameLoopFiles/BP_checkpoints.BP_checkpoints_C" (`KismetMathLibrary.MakeTransform` (0.0 0.0 0.0)) "Undefined" "MultiplyWithRoot" null null))
      (`BlueprintMapLibrary.Map_Add` (`self.CustomerMap`) (`self.id`) _returnvalue))))

(event `self.ReceiveBeginPlay`
  (set `DA_CustomerList.Customers` (`self.CustomerMap`) (`self.CustomerListDataAsset`)))

(event `self.ReceiveEndPlay`
  (params (EndPlayReason :type "EEndPlayReason Enum" :default "Destroyed"))
  (`BlueprintMapLibrary.Map_Clear` (`DA_CustomerList.Customers` (`self.CustomerListDataAsset`))))

(fn `UserConstructionScript`)