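; Pizza order manager Blueprint that sets up the pizza orders when RequestOrder is called.
; RequestOrder initialises the MPizzas object, then InitiateOrders loops over an array to fill its MPizzasStruct with pizza structs keyed by index.
; An unconnected branch, which never runs, would check the order limit, queue random customers and spawn Pizza actors into MPizzas.
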(event `self.RequestOrder`
  (`DA_Pizzas.Initialise` (`self.mPizzas`))
  (`self.InitiateOrders`))

(event `self.InitiateOrders`
  ;[1 1 1] Use that array to generate the pizzas
  (for (_ _array_index) _
    (`BlueprintMapLibrary.Map_Add` (`DA_Pizzas.mPizzasStruct` (`self.mPizzas`)) _array_index (make `PizzaStruct` 100))))

(fn `UserConstructionScript`)