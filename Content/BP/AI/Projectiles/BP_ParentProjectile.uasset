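; Base AI projectile that is lobbed at a target and damages customer orders when it hits the parkour player.
; On BeginPlay it plays a sound and sets a suggested launch velocity, aiming at the target's location offset by its velocity plus random scatter.
; A looping timer tumbles it toward a random rotation.
; Overlapping a ParkourPlayerInterface actor deals damage through the customer subsystem and destroys the projectile.
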(event `self.ReceiveBeginPlay`
  (bind _returnvalue (`KismetMathLibrary.RandomFloatInRange` -180.0 180.0))
  (bind _target (`self.target`))
  (bind _projectilemovement (`self.ProjectileMovement`))
  (bind (_startpos _endpos _launchspeed) (`self.CalculateProjectileVelocity` _target))
  ;[0 0 0] Calculate the Velocity on Begin play
  (`/Engine/EditorBlueprintResources/StandardMacros.IsValid` _target
    (:`Is Valid`
      (`GameplayStatics.PlaySoundAtLocation` (`self.Sound`) (`self.K2_GetActorLocation`) (struct) 1.0 1.0 0.0 null null null null)
      (bind _tossvelocity (`GameplayStatics.BlueprintSuggestProjectileVelocity` _startpos _endpos _launchspeed 0.0 "DoNotTrace"))
      (set `MovementComponent.Velocity` _tossvelocity _projectilemovement)
      (set `ProjectileMovementComponent.bRotationFollowsVelocity` true _projectilemovement)
      ;[0 0 0] Find a random rotation direction and start rotation
      (set `self.rotDirection` (`KismetMathLibrary.MakeRotator` _returnvalue _returnvalue _returnvalue))
      (`KismetSystemLibrary.K2_SetTimerDelegate` (delegate `Rotate`) (`self.rate`) true))))

(event `Rotate`
  ;[0 0 0] Find a random rotation direction and start rotation
  (`self.K2_AddActorLocalRotation` (`KismetMathLibrary.RLerp` (`self.K2_GetActorRotation`) (`self.rotDirection`) (`GameplayStatics.GetTimeSeconds`))))

(event `self.Collider.OnComponentBeginOverlap`
  (params (OverlappedComponent :type "PrimitiveComponent Object Reference") (OtherActor :type "Actor Object Reference") (OtherComp :type "PrimitiveComponent Object Reference") (OtherBodyIndex :type Integer) (bFromSweep :type Boolean) (SweepResult :type "HitResult Structure (by ref)"))
  ;[0 0 0] When the Projectile overlaps, it deals damage to the orders, and Destroys
  (if (`KismetSystemLibrary.DoesImplementInterface` OtherActor "/Script/GroupProj27.ParkourPlayerInterface")
    (`CustomerSubsystem.DealDamageToOrders` (subsystem `CustomerSubsystem`) (`self.DamageValue`))
    (`self.K2_DestroyActor`)))

(fn `UserConstructionScript`)