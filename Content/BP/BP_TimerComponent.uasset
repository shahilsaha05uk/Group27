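; BP_TimerComponent runs a countdown timer and reports it through a clock subsystem.
; On BeginPlay it binds StartTimer to the subsystem's start event, which resets the current time to the total and starts a looping timer.
; Each tick of that timer subtracts the rate and broadcasts the formatted time string.
; At zero it calls the subsystem's stop on every loop, as the stored timer handle is never cleared here.
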(event `self.ReceiveBeginPlay`
  (add `ClockSubsystem.StartTimer` (subsystem `ClockSubsystem`) (delegate `StartTimer`)))

(event `StartTimer`
  (set `self.cTime` (`self.TotalTime`))
  (bind _returnvalue (`KismetSystemLibrary.K2_SetTimerDelegate` (delegate `Countdown`) (`self.rate`) true))
  (set `self.CountdownHandler` _returnvalue))

(event `Countdown`
  (if (> (`self.cTime`) 0.0)
    (bind _output_get (set `self.cTime` (- (`self.cTime`) (`self.rate`))))
    (`ClockSubsystem.CurrentTime` (subsystem `ClockSubsystem`) (`KismetStringLibrary.TimeSecondsToString` _output_get))
    (else
      (`ClockSubsystem.StopTimer` (subsystem `ClockSubsystem`)))))