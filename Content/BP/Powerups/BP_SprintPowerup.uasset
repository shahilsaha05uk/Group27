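; BP_SprintPowerup is a powerup that temporarily changes the walk speed of the actor that collided with it.
; On activation it calls the parent logic, gets the movement component through a message call, saves its MaxWalkSpeed and sets it to RunSpeed.
; A short one-shot timer then triggers deactivation, which restores the saved speed and clears the collided actor reference.
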(event `self.ActivatePowerup`
  (`parent.ActivatePowerup`)
  (bind _returnvalue (message `ParkourPlayerInterface.GetMovementComp` (`self.collidedActor`)))
  (set `self.defaultSpeed` (`CharacterMovementComponent.MaxWalkSpeed` _returnvalue))
  (set `CharacterMovementComponent.MaxWalkSpeed` (`self.RunSpeed`) _returnvalue)
  (bind _returnvalue_2 (`KismetSystemLibrary.K2_SetTimerDelegate` (delegate `Sprinting`) 2.0))
  (set `self.SprintTimeHandler` _returnvalue_2))

(event `Sprinting`
  (`KismetSystemLibrary.K2_ClearAndInvalidateTimerHandle` (`self.SprintTimeHandler`))
  (`self.DeactivatePowerup`))

(event `self.DeactivatePowerup`
  (bind _returnvalue (message `ParkourPlayerInterface.GetMovementComp` (`self.collidedActor`)))
  (set `CharacterMovementComponent.MaxWalkSpeed` (`self.defaultSpeed`) _returnvalue)
  (set `self.collidedActor` null))

(fn `UserConstructionScript`
  (`parent.UserConstructionScript`))