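; BP_InputController is a player controller that spawns the player and shows the end-of-match screen.
; On BeginPlay it binds to BP_GameLevelMode's OnDecisionMade, sets game-only input, then spawns and possesses a BP_ParentPlayer at the player start.
; When a decision fires, it switches to UI-only input, shows the cursor and adds WBP_WinScreen with that decision.
; A debug O key release triggers a LOSE decision through the game mode.
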(event `self.ReceiveBeginPlay`
  ;[0 0 0] Spawning the Player
  (`parent.ReceiveBeginPlay`)
  (bind _asbp_game_level_mode (cast `/Game/BP/GameModes/BP_GameLevelMode` (`GameplayStatics.GetGameMode`)))
  (add `GameLevelMode.OnDecisionMade` _asbp_game_level_mode (`|CreateDelegate` :!event `OnDecisionMade`))
  (`WidgetBlueprintLibrary.SetInputMode_GameOnly` self)
  (bind _returnvalue (`|SpawnActorFromClass` "/Game/BP/BP_ParentPlayer.BP_ParentPlayer_C" (`self.GetTransform` (`GameModeBase.K2_FindPlayerStart` (`GameplayStatics.GetGameMode`) self "")) "Undefined" "MultiplyWithRoot" null null))
  (bind _output_get (set `self.mPawn` _returnvalue))
  (`self.Possess` _output_get))

(event `OnDecisionMade`
  (params (Decision :type "EGameDecision Enum" :default "LOSE"))
  ;[0 0 0] OnDecisionMade
  (`WidgetBlueprintLibrary.SetInputMode_UIOnlyEx` self null)
  (set `self.bShowMouseCursor` true)
  (bind _returnvalue (`|CreateWidget` "/Game/Widgets/WBP_WinScreen.WBP_WinScreen_C" null Decision))
  (`UserWidget.AddToViewport` _returnvalue 0))

(event `Key|O`
  (params (Key :type "Key Structure"))
  ;[1 0.8953 0] DEBUG!!
  (:`Released`
    (bind _asbp_game_level_mode (cast `/Game/BP/GameModes/BP_GameLevelMode` (`GameplayStatics.GetGameMode`)))
    (`GameLevelMode.OnDecisionMade` _asbp_game_level_mode "LOSE")))

(fn `UserConstructionScript`)