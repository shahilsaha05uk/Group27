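; Pizza actor component with a function that generates a fresh, random-sized batch of pizza orders through the customer subsystem.
; InitiateOrders clears the order list, creates each order with default quality and decay values, then pushes the list back to the subsystem.
; The customer list is shuffled but never read, as loop indices serve as customer and pizza IDs.
; An auto-initialise flag triggers the subsystem's order-initialised call; otherwise it returns true.
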(fn `InitiateOrders`
  (params (AutoInitialise :type Boolean))
  (returns (ReturnValue :type Boolean))
  (bind _returnvalue (`CustomerSubsystem.GetOrderList` (subsystem `CustomerSubsystem`)))
  (`BlueprintMapLibrary.Map_Clear` _returnvalue)
  (bind _values (`BlueprintMapLibrary.Map_Values` (`CustomerSubsystem.GetAllCustomers` (subsystem `CustomerSubsystem`))))
  (`KismetArrayLibrary.Array_Shuffle` _values)
  (for _index (range (+ (`KismetMathLibrary.RandomIntegerInRange` 1 6) 1))
    (`self.CreateOrder` _index (make `PizzaStruct` _index 100 1)))
  (`CustomerSubsystem.UpdateOrders` (subsystem `CustomerSubsystem`) _returnvalue)
  (if (`local.AutoInitialise`)
    (`CustomerSubsystem.OnOrderInitialised` (subsystem `CustomerSubsystem`))
    (else
      (return true))))