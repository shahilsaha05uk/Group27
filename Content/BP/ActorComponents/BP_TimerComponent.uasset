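; Actor component that runs a looping countdown timer and reports its state and time through a clock subsystem.
; On BeginPlay it binds to the subsystem's start, finish and stop events and sets the status to idle.
; Each tick of the timer subtracts the rate, broadcasts the remaining time as a formatted string, and signals finish at zero.
; Start, stop and finish update the clock status and manage the timer handle.
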(event `self.ReceiveBeginPlay`
  (bind _returnvalue (subsystem `ClockSubsystem`))
  (add `ClockSubsystem.StartTimer` _returnvalue (delegate `StartTimer`))
  ;[0 0 0] When the Timer finishes without interruption
  (add `ClockSubsystem.FinishTimer` _returnvalue (delegate `FinishTimer`))
  ;[0 0 0] When the Stop Timer is invoked
  (add `ClockSubsystem.StopTimer` _returnvalue (delegate `StopTimer`))
  ;[0 0 0] Initial State
  (`ClockSubsystem.SetClockStatus` (subsystem `ClockSubsystem`) "TIMER_IDLE"))

(event `StopTimer`
  ;[0 0 0] When the Stop Timer is invoked
  (`KismetSystemLibrary.K2_ClearAndInvalidateTimerHandle` (`self.CountdownHandler`))
  (`ClockSubsystem.SetClockStatus` (subsystem `ClockSubsystem`) "TIMER_INTERRUPTED"))

(event `FinishTimer`
  ;[0 0 0] When the Timer finishes without interruption
  (`KismetSystemLibrary.K2_ClearAndInvalidateTimerHandle` (`self.CountdownHandler`))
  (`ClockSubsystem.SetClockStatus` (subsystem `ClockSubsystem`) "TIMER_FINISHED"))

(event `StartTimer`
  ;[0 0 0] When the Start timer is Invoked
  (set `self.cTime` (`self.TotalTime`))
  (bind _returnvalue (`KismetSystemLibrary.K2_SetTimerDelegate` (delegate `Countdown`) (`self.rate`) true))
  (set `self.CountdownHandler` _returnvalue)
  (`ClockSubsystem.SetClockStatus` (subsystem `ClockSubsystem`) "TIMER_RUNNING"))

(event `Countdown`
  ;[0 0 0] Perform countdown
  (if (> (`self.cTime`) 0.0)
    (bind _output_get (set `self.cTime` (`KismetMathLibrary.FClamp` (- (`self.cTime`) (`self.rate`)) 0.0 100000.0)))
    (`ClockSubsystem.CurrentTime` (subsystem `ClockSubsystem`) (`KismetStringLibrary.TimeSecondsToString` _output_get))
    (else
      ;[0 0 0] Clear the Handler when the current time reaches 0
      (`ClockSubsystem.FinishTimer` (subsystem `ClockSubsystem`)))))