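; BP_InputController is a player controller that spawns and possesses the player's pawn and sets up their HUD.
; On BeginPlay it spawns the game mode's default pawn at a player start, possesses it and adds a WBP_testPlayerHUD widget to the viewport.
; Releasing the 1 key asks the pizza manager on BP_GameLevelMode to request an order.
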(event `self.ReceiveBeginPlay`
  (bind _returnvalue (`GameplayStatics.GetGameMode`))
  ;[0 0 0] Spawning the Player
  (`parent.ReceiveBeginPlay`)
  (bind _returnvalue_2 (`|SpawnActorFromClass` (`GameModeBase.DefaultPawnClass` _returnvalue) (`self.GetTransform` (`GameModeBase.K2_FindPlayerStart` _returnvalue self "")) "Undefined" "MultiplyWithRoot" null null))
  (bind _output_get (set `self.mPawn` _returnvalue_2))
  (`self.Possess` _output_get)
  (bind _returnvalue_3 (`|CreateWidget` "/Game/Prototypes/Shahil/GameLoopFiles/WBP_testPlayerHUD.WBP_testPlayerHUD_C" self))
  (`UserWidget.AddToViewport` _returnvalue_3 0))

(event `Key|One`
  (params (Key :type "Key Structure"))
  (:`Released`
    (bind _asbp_game_level_mode (cast `/Game/BP/BP_GameLevelMode` (`GameplayStatics.GetGameMode`)))
    (`PizzaManager.RequestOrder` (`GameLevelMode.mPizzaManager` _asbp_game_level_mode))))

(fn `UserConstructionScript`)