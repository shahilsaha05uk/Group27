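; BP_GameLevelMode is the level mode for a pizza delivery game, generating a batch of customer orders on request.
; RequestforOrders shuffles all BP_checkpoints actors and creates full-quality orders in the PizzaSubsystem for a random number of them.
; Customers implementing Bi_checkpointInterface receive an order message, then the subsystem broadcasts initialisation and starts a looping quality-decay timer.
; The OnPlayerIsLate event is an empty stub.
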(event `PizzaModeInterface.RequestForOrders`
  (bind _returnvalue (subsystem `PizzaSubsystem`))
  ;[0.6469 0.5865 0] Needs to be worked on
  (bind _outactors (`GameplayStatics.GetAllActorsOfClass` "/Game/Prototypes/Shahil/GameLoopFiles/BP_checkpoints.BP_checkpoints_C"))
  (bind _output_get (set `self.Checkpoint Actors` _outactors))
  (`KismetArrayLibrary.Array_Shuffle` _output_get)
  (for _index (range (+ (`KismetMathLibrary.RandomIntegerInRange` 1 6) 1))
    (bind _customerid (`/Game/Prototypes/Shahil/GameLoopFiles/BP_checkpoints.CustomerID` (`|GetArrayItem` (`self.Checkpoint Actors`) _index)))
    (`PizzaSubsystem.CreateOrder` _returnvalue _customerid (make `PizzaStruct` null 100))
    (bind _returnvalue_2 (`PizzaSubsystem.GetCustomer` _returnvalue _customerid))
    (if (`KismetSystemLibrary.DoesImplementInterface` _returnvalue_2 "/Game/Prototypes/Shahil/GameLoopFiles/bi_checkpointInterface.bi_checkpointInterface_C")
      (message `/Game/Prototypes/Shahil/GameLoopFiles/bi_checkpointInterface.InitOrder` _returnvalue_2)))
  (`PizzaSubsystem.OnOrderInitialised` _returnvalue)
  (`PizzaSubsystem.StartQualityTimer` _returnvalue 0.5 1 true))

(event `self.OnPlayerIsLate`
  (params (bHasArrived :type Boolean)))

(fn `UserConstructionScript`)